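; Procedural city actor that builds a river, bridges, ground, buildings and riverside trees in its construction script.
; SplineRiver drives spline meshes, instanced bridges at its points and instanced trees scattered along both banks.
; A grid places individual building meshes with random tints and heights that taper from the center, skipping the center and cells near the river.
; Building and tree variation draws from a random stream, and the ground plane scales to the grid.
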(event EventBeginPlay)

(event Collision|EventActorBeginOverlap
  (params (OtherActor :type Actor%20Object%20Reference)))

(event EventTick
  (params (DeltaSeconds :type Float%20%28single-precision%29)))

(fn ConstructionScript
  (bind _rndstream (Variables|Default|GetrndStream))
  (bind _buildingscalerange (Variables|Default|GetBuildingScaleRange))
  (bind _distance (Variables|Default|GetDistance))
  (bind _rndstream_2 (Variables|Default|GetrndStream))
  (bind _rowcols (Variables|Default|GetRowCols))
  (bind _rowcols_2 (Variables|Default|GetRowCols))
  (bind _spline_river (Variables|Default|GetSpline_River))
  (bind _ism_trees (Variables|Default|GetISM_Trees))
  (bind _spline_river_2 (Variables|Default|GetSpline_River))
  (bind _rndstream_3 (Variables|Default|GetrndStream))
  (bind _treescount (Variables|Default|GetTreesCount))
  (bind _rndstream_4 (Variables|Default|GetrndStream))
  (bind _distance_2 (Variables|Default|GetDistance))
  (bind _returnvalue (Math|Random|RandomFloatinRangefromStream 6e+02 3.5e+02 _rndstream_4))
  (bind _returnvalue_2 (Math|Random|RandomFloatinRangefromStream 0.25 0.5 _rndstream))
  (bind _returnvalue_3 (Math|Random|RandomFloatinRangefromStream 0.25 0.5 _rndstream_3))
  (bind _returnvalue_4 (Math|Random|RandomFloatinRangefromStream (.x _buildingscalerange) (.y _buildingscalerange) _rndstream_2))
  (bind _returnvalue_5 (* _distance 0.01))
  (Utilities|FlowControl|Sequence
    (:then_0
      ;[1 1 1] River
      (for _index (range 0 (- (Spline|GetNumberOfSplinePoints _spline_river) 1))
        (bind _returnvalue_6 (AddComponent|AddSplineMeshComponent false))
        (SplineMesh|SetStartandEnd _returnvalue_6 (.Location (Spline|GetLocationandTangentatSplinePoint _spline_river _index "Local")) (.Tangent (Spline|GetLocationandTangentatSplinePoint _spline_river _index "Local")) (.Location (Spline|GetLocationandTangentatSplinePoint _spline_river (+ _index 1) "Local")) (.Tangent (Spline|GetLocationandTangentatSplinePoint _spline_river (+ _index 1) "Local")) true :!class /Script/Engine.SplineMeshComponent)
        ;[1 1 1] Bridges
        (Components|InstancedStaticMesh|AddInstance (Variables|Default|GetISM_Bridges) (Math|Transform|MakeTransform (.Location (Spline|GetLocationandTangentatSplinePoint _spline_river _index "Local")) (Math|Conversions|RotationFromXVector (.Tangent (Spline|GetLocationandTangentatSplinePoint _spline_river _index "Local"))) "1,1,1"))))
    (:then_1
      ;[1 1 1] Ground
      (Variables|Default|Setorigin (* _rowcols_2 (Math|Vector2D|MakeVector2D _distance _distance) "(X=0.500000,Y=0.500000)"))
      (Transformation|SetRelativeScale3D (Variables|Default|GetPlane) (Math|Conversions|ToVector(Vector2D) (* (+ _rowcols_2 "(X=2.000000,Y=2.000000)") (Math|Vector2D|MakeVector2D _returnvalue_5 _returnvalue_5)) 1.0)))
    (:then_2
      ;[1 1 1] Buildings
      (for _index_2 (range 0 (Math|Float|Truncate (.x _rowcols)))
        (for _index_3 (range 0 (Math|Float|Truncate (.y _rowcols)))
          (Variables|Default|Setheight (* (Math|Float|MapRangeClamped (Math|Vector|Distance(Vector) "0, 0, 0" (- (Math|Vector|MakeVector (* _index_2 _distance_2) (* _index_3 _distance_2) (* (Variables|Default|Getheight) 5e+01)) (Math|Conversions|ToVector(Vector2D) (Variables|Default|Getorigin)))) 0.0 6e+03 2.0 0.4) (Math|Random|RandomFloatinRangefromStream 0.5 5.0 (Variables|Default|GetrndStream))))
          (if (not (or (Math|Vector|Equal(Vector) (- (Math|Vector|MakeVector (* _index_2 _distance_2) (* _index_3 _distance_2) (* (Variables|Default|Getheight) 5e+01)) (Math|Conversions|ToVector(Vector2D) (Variables|Default|Getorigin))) (Math|Vector|MakeVector 0.0 0.0 (* (Variables|Default|Getheight) 5e+01)) 0.0001) (< (Math|Vector|Distance(Vector) (Spline|FindLocationClosesttoWorldLocation (Variables|Default|GetSpline_River) (- (Math|Vector|MakeVector (* _index_2 _distance_2) (* _index_3 _distance_2) (* (Variables|Default|Getheight) 5e+01)) (Math|Conversions|ToVector(Vector2D) (Variables|Default|Getorigin))) "Local") (- (Math|Vector|MakeVector (* _index_2 _distance_2) (* _index_3 _distance_2) (* (Variables|Default|Getheight) 5e+01)) (Math|Conversions|ToVector(Vector2D) (Variables|Default|Getorigin)))) (Variables|Default|GetSplineOffset))))
            (bind _returnvalue_7 (AddComponent|AddStaticMeshComponent false (Math|Transform|MakeTransform (- (Math|Vector|MakeVector (* _index_2 _distance_2) (* _index_3 _distance_2) (* (Variables|Default|Getheight) 5e+01)) (Math|Conversions|ToVector(Vector2D) (Variables|Default|Getorigin))) "0, 0, 0" (Math|Vector|MakeVector _returnvalue_4 _returnvalue_4 (Variables|Default|Getheight)))))
            (bind _returnvalue_8 (Rendering|Material|CreateDynamicMaterialInstance _returnvalue_7 0 "/Game/Materials/OpaqueMaster.OpaqueMaster" "None" :!class /Script/Engine.PrimitiveComponent))
            (Rendering|Material|SetVectorParameterValue _returnvalue_8 "Color" (Math|Conversions|ToLinearColor(Vector) (* (+ (Math|Random|RandomUnitVectorfromStream (Variables|Default|GetrndStream)) 0.5) 0.5)) :!class /Script/Engine.MaterialInstanceDynamic)))))
    (:then_3
      ;[1 1 1] Trees
      (for _index_4 (range 0 _treescount)
        (Components|InstancedStaticMesh|AddInstance _ism_trees (Math|Transform|MakeTransform (+ (Spline|GetLocationatDistanceAlongSpline _spline_river_2 (* _index_4 (/ (Spline|GetSplineLength _spline_river_2) (Math|Conversions|ToFloat(Integer) _treescount))) "Local") (Math|Vector|RotateVector (Math|Vector|MakeVector 0.0 (* _returnvalue -1.0) 0.0) (Math|Conversions|RotationFromXVector (Spline|GetTangentatDistanceAlongSpline _spline_river_2 (* _index_4 (/ (Spline|GetSplineLength _spline_river_2) (Math|Conversions|ToFloat(Integer) _treescount))) "Local")))) "0, 0, 0" (Math|Vector|MakeVector _returnvalue_3 _returnvalue_3 (Math|Random|RandomFloatinRangefromStream 0.25 0.75 _rndstream_3))))
        (Components|InstancedStaticMesh|AddInstance _ism_trees (Math|Transform|MakeTransform (+ (Spline|GetLocationatDistanceAlongSpline _spline_river_2 (* _index_4 (/ (Spline|GetSplineLength _spline_river_2) (Math|Conversions|ToFloat(Integer) _treescount))) "Local") (Math|Vector|RotateVector (Math|Vector|MakeVector 0.0 _returnvalue 0.0) (Math|Conversions|RotationFromXVector (Spline|GetTangentatDistanceAlongSpline _spline_river_2 (* _index_4 (/ (Spline|GetSplineLength _spline_river_2) (Math|Conversions|ToFloat(Integer) _treescount))) "Local")))) "0, 0, 0" (Math|Vector|MakeVector _returnvalue_2 _returnvalue_2 (Math|Random|RandomFloatinRangefromStream 0.25 0.75 _rndstream))))))))